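; BP_Plant1 is an interactable potted plant that can be watered once to advance the "WaterPlants" task.
; Focus toggles custom depth on the dirt, plant and pot meshes.
; Interaction swaps the dirt to a watered material and plays a timeline that bounces the plant's scale relative to its starting size.
; When the bounce finishes, it increments the task through BP_FirstPersonGameMode.
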(event `self.ReceiveBeginPlay`
  (set `self.OriginalScale` (`SceneComponent.RelativeScale3D` (`self.plant`))))

(event `self.Interface_ToggleFocus`
  (params (Focus :type Boolean))
  (`PrimitiveComponent.SetRenderCustomDepth` (`self.dirt`) Focus)
  (`PrimitiveComponent.SetRenderCustomDepth` (`self.plant`) Focus)
  (`PrimitiveComponent.SetRenderCustomDepth` (`self.pot`) Focus))

(event `/Game/Dynamic/Interaction/BPI_Interaction.Interaction`
  (if (not (`self.bisWatered`))
    (`PrimitiveComponent.SetMaterial` (`self.dirt`) 0 "/Game/Static/Materials/M_WateredDirt.M_WateredDirt")
    (set `self.bisWatered` true)
    (bind (_direction _scalemult) (`Timeline|TL_Bounce`)
      (:`Update`
        (`SceneComponent.SetRelativeScale3D` (`self.plant`) (`KismetMathLibrary.MakeVector` (* (.x (`self.OriginalScale`)) _scalemult) (* (.y (`self.OriginalScale`)) _scalemult) (* (.z (`self.OriginalScale`)) _scalemult))))
      (:`Finished`
        (bind _asbp_first_person_game_mode (cast `/Game/Dynamic/FirstPerson/Blueprints/BP_FirstPersonGameMode` (`GameplayStatics.GetGameMode`)))
        (`/Game/Dynamic/FirstPerson/Blueprints/BP_FirstPersonGameMode.IncrementTaskByID` _asbp_first_person_game_mode "WaterPlants" 1)))))

(fn `GetInteractionName`
  (returns (InteractionName :type String))
  (return ""))

(fn `GetInteractionWidgetRef`
  (returns (Ref :type "WidgetComponent Object Reference"))
  (return (`self.Widget`)))

(fn `UserConstructionScript`)