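; BP_Plant4 is an interactable plant that the player can water once as part of a "WaterPlants" task.
; Focus toggles the plant's custom depth rendering, and interaction shows the Dirt component and sets a watered flag that blocks repeats.
; A timeline then scales the plant from its BeginPlay scale and, when finished, increments the task through BP_FirstPersonGameMode.
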(event `self.ReceiveBeginPlay`
  (set `self.OriginalScale` (`SceneComponent.RelativeScale3D` (`self.plant`))))

(event `self.Interface_ToggleFocus`
  (params (Focus :type Boolean))
  (`PrimitiveComponent.SetRenderCustomDepth` (`self.plant`) Focus))

(event `/Game/Dynamic/Interaction/BPI_Interaction.Interaction`
  (if (not (`self.bisWatered`))
    (`KismetSystemLibrary.PrintString` "Plant has been watered!")
    (`SceneComponent.SetVisibility` (`self.Dirt`) true false)
    (set `self.bisWatered` true)
    (bind (_direction _scalemult) (`Timeline|Timeline`)
      (:`Update`
        (`SceneComponent.SetRelativeScale3D` (`self.plant`) (`KismetMathLibrary.MakeVector` (* (.x (`self.OriginalScale`)) _scalemult) (* (.y (`self.OriginalScale`)) _scalemult) (* (.z (`self.OriginalScale`)) _scalemult))))
      (:`Finished`
        (bind _asbp_first_person_game_mode (cast `/Game/Dynamic/FirstPerson/Blueprints/BP_FirstPersonGameMode` (`GameplayStatics.GetGameMode`)))
        (`/Game/Dynamic/FirstPerson/Blueprints/BP_FirstPersonGameMode.IncrementTaskByID` _asbp_first_person_game_mode "WaterPlants" 1)))
    (else
      (`KismetSystemLibrary.PrintString` "Plants already waterd!"))))

(fn `GetInteractionName`
  (returns (InteractionName :type String))
  (return ""))

(fn `GetInteractionWidgetRef`
  (returns (Ref :type "WidgetComponent Object Reference"))
  (return (`self.Widget`)))

(fn `UserConstructionScript`)