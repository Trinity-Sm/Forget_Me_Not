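; BP_InteractionArea is an interaction proxy actor that relays focus and interaction to the actor it belongs to.
; Focus changes are stored, forwarded to the parent actor, and used to show or hide that parent's interaction widget.
; Interaction goes to the attach parent actor if it implements BPI_Interaction, otherwise to that actor's ChildActorComponent if the component implements it.
; It names itself InteractionArea and returns no widget of its own.
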(event `ToggleFocus`
  (params (Focused :type Boolean))
  (set `self.Focused` Focused)
  (message `/Game/Dynamic/Interaction/BPI_Interaction.Interface_ToggleFocus` (`self.GetParentActor`) (`self.Focused`))
  (bind _ref (message `/Game/Dynamic/Interaction/BPI_Interaction.GetInteractionWidgetRef` (`self.GetParentActor`)))
  (`SceneComponent.SetHiddenInGame` _ref (not (`self.Focused`)) false))

(event `/Game/Dynamic/Interaction/BPI_Interaction.Interaction`
  (bind _returnvalue (`self.GetAttachParentActor`))
  (bind _returnvalue_2 (`self.GetComponentByClass` _returnvalue "/Script/Engine.ChildActorComponent"))
  (if (`KismetSystemLibrary.DoesImplementInterface` _returnvalue "/Game/Dynamic/Interaction/BPI_Interaction.BPI_Interaction_C")
    (message `/Game/Dynamic/Interaction/BPI_Interaction.Interaction` _returnvalue)
    (elif (`KismetSystemLibrary.DoesImplementInterface` _returnvalue_2 "/Game/Dynamic/Interaction/BPI_Interaction.BPI_Interaction_C")
      (message `/Game/Dynamic/Interaction/BPI_Interaction.Interaction` _returnvalue_2))))

(fn `GetInteractionName`
  (returns (InteractionName :type String))
  (return (`self.InteractionArea`)))

(fn `GetInteractionWidgetRef`
  (returns (Ref :type "WidgetComponent Object Reference"))
  (return null))

(fn `UserConstructionScript`)