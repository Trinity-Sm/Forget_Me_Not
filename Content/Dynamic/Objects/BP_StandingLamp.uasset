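; BP_StandingLamp is an interactable lamp that the player can switch on and off.
; Focus changes toggle custom depth rendering on the TableLamp component, typically used for highlighting.
; Each interaction alternates the PointLight visibility through a FlipFlop, with the first one setting it visible.
; Its interaction getters return InteractionArea for the name and nothing for the widget reference.
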(event `/Game/Dynamic/Interaction/BPI_Interaction.Interface_ToggleFocus`
  (params (Focus :type Boolean))
  (`PrimitiveComponent.SetRenderCustomDepth` (`self.TableLamp`) Focus))

(event `/Game/Dynamic/Interaction/BPI_Interaction.Interaction`
  (bind _pointlight (`self.PointLight`))
  (`/Engine/EditorBlueprintResources/StandardMacros.FlipFlop`
    (:`A`
      (`SceneComponent.SetVisibility` _pointlight true false))
    (:`B`
      (`SceneComponent.SetVisibility` _pointlight false false))))

(fn `GetInteractionName`
  (returns (InteractionName :type String))
  (return (`self.InteractionArea`)))

(fn `GetInteractionWidgetRef`
  (returns (Ref :type "WidgetComponent Object Reference"))
  (return null))

(fn `UserConstructionScript`)