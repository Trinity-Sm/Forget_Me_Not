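; BP_CuttingBoard is an interactable cutting board whose Food mesh becomes a chopped carrot when used.
; BeginPlay reads SavedDay from the day game instance and makes Food visible on days 2 and 3.
; Interaction increments the game mode's CutCarrot task, then resets Food's relative transform and swaps its mesh.
; Interface focus toggles custom depth on the Sink and Food components.
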(event `self.Interface_ToggleFocus`
  (params (Focus :type Boolean))
  (`PrimitiveComponent.SetRenderCustomDepth` (`self.Sink`) Focus)
  (`PrimitiveComponent.SetRenderCustomDepth` (`self.Food`) Focus))

(event `self.Interaction`
  (bind _food (`self.Food`))
  (bind _asbp_first_person_game_mode (cast `/Game/Dynamic/FirstPerson/Blueprints/BP_FirstPersonGameMode` (`GameplayStatics.GetGameMode`)))
  (`/Game/Dynamic/FirstPerson/Blueprints/BP_FirstPersonGameMode.IncrementTaskByID` _asbp_first_person_game_mode "CutCarrot" 1)
  (`SceneComponent.K2_SetRelativeLocationAndRotation` _food (0.0 0.0 12.0) (struct) false false)
  (`StaticMeshComponent.SetStaticMesh` _food "/Game/Static/Assets/Kitchen/food_ingredient_carrot_chopped.food_ingredient_carrot_chopped"))

(event `self.ReceiveBeginPlay`
  (bind _asbp_game_instance_game_day (cast `/Game/Dynamic/BP_GameInstance_GameDay` (`GameplayStatics.GetGameInstance`)))
  (switch `int` (`/Game/Dynamic/BP_GameInstance_GameDay.SavedDay` _asbp_game_instance_game_day)
    (:`2`
      _)
    (:`3`
      _))
  (`SceneComponent.SetVisibility` (`self.Food`) true false))

(fn `GetInteractionName`
  (returns (InteractionName :type String))
  (return ""))

(fn `GetInteractionWidgetRef`
  (returns (Ref :type "WidgetComponent Object Reference"))
  (return null))

(fn `UserConstructionScript`)