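; Interactable light switch that forwards the player's interaction to the lights listed in LightsToControl.
; Focus toggles custom depth rendering on the switch mesh for highlighting.
; Each interaction uses a FlipFlop to rotate the switch between two positions, then calls Interaction on every linked light, which handles its own response.
; It reports InteractionArea as its interaction name and supplies no interaction widget.
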(event `self.Interface_ToggleFocus`
  (params (Focus :type Boolean))
  (`PrimitiveComponent.SetRenderCustomDepth` (`self.LightSwitch`) Focus))

(event `self.Interaction`
  (bind _actualswitch (`self.actualSwitch`))
  (`/Engine/EditorBlueprintResources/StandardMacros.FlipFlop`
    (:`A`
      (`SceneComponent.K2_SetRelativeRotation` _actualswitch (struct :`Roll` -140.0) false false))
    (:`B`
      (`SceneComponent.K2_SetRelativeRotation` _actualswitch (struct :`Roll` 140.0) false false)))
  (for _array_element (`self.LightsToControl`)
    (`/Game/Dynamic/Interaction/BPI_Interaction.Interaction` _array_element)))

(fn `GetInteractionName`
  (returns (InteractionName :type String))
  (return (`self.InteractionArea`)))

(fn `GetInteractionWidgetRef`
  (returns (Ref :type "WidgetComponent Object Reference"))
  (return null))

(fn `UserConstructionScript`)