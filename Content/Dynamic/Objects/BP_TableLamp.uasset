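; Interactable table lamp whose point light is switched on and off by the player's interaction.
; BeginPlay shows the light if InitiallyOn is set, and interface focus toggles custom depth on the lamp mesh.
; Interaction alternates visibility through a FlipFlop that always starts with "on", independent of InitiallyOn, so a lit lamp's first interaction changes nothing.
; The interaction name getter returns InteractionArea, while the widget getter returns nothing.
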(event `self.ReceiveBeginPlay`
  (if (`self.InitiallyOn`)
    (`SceneComponent.SetVisibility` (`self.PointLight`) true false)))

(event `/Game/Dynamic/Interaction/BPI_Interaction.Interface_ToggleFocus`
  (params (Focus :type Boolean))
  (`PrimitiveComponent.SetRenderCustomDepth` (`self.TableLamp`) Focus))

(event `/Game/Dynamic/Interaction/BPI_Interaction.Interaction`
  (bind _pointlight (`self.PointLight`))
  (`/Engine/EditorBlueprintResources/StandardMacros.FlipFlop`
    (:`A`
      (`SceneComponent.SetVisibility` _pointlight true false))
    (:`B`
      (`SceneComponent.SetVisibility` _pointlight false false))))

(fn `GetInteractionName`
  (returns (InteractionName :type String))
  (return (`self.InteractionArea`)))

(fn `GetInteractionWidgetRef`
  (returns (Ref :type "WidgetComponent Object Reference"))
  (return null))

(fn `UserConstructionScript`)