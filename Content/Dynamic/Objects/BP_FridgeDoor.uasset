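; Interactable fridge door that toggles open and closed each time it receives an Interaction event.
; A FlipFlop alternates between playing and reversing a timeline, whose float lerps the door mesh's relative location and yaw to swing and shift it open.
; Each interaction plays a pickup sound, and the name getter returns the InteractionArea component while the widget getter returns nothing.
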(event `/Game/Dynamic/Interaction/BPI_Interaction.Interaction`
  (`GameplayStatics.PlaySoundAtLocation` "/Engine/VREditor/Sounds/UI/Object_PickUp.Object_PickUp" (0.0 0.0 0.0) (struct) 1.0 1.0 0.0 null null null null)
  (`/Engine/EditorBlueprintResources/StandardMacros.FlipFlop`
    (:`A`
      (bind (_direction _doorfloat) (`Timeline|OpenDoor Timeline` :!via `PlayFromStart` :!label _label)
        (:`Update`
          (`SceneComponent.K2_SetRelativeLocationAndRotation` (`self.FridgeDoor`) (`KismetMathLibrary.MakeVector` (`KismetMathLibrary.Lerp` 0.0 -20.0 _doorfloat) (`KismetMathLibrary.Lerp` 0.0 140.0 _doorfloat) 240.0) (`KismetMathLibrary.MakeRotator` 0.0 -180.0 (`KismetMathLibrary.Lerp` 0.0 90.0 _doorfloat)) false false))))
    (:`B`
      (goto _label :!via `Reverse`))))

(fn `GetInteractionName`
  (returns (InteractionName :type String))
  (return (`self.InteractionArea`)))

(fn `GetInteractionWidgetRef`
  (returns (Ref :type "WidgetComponent Object Reference"))
  (return null))

(fn `UserConstructionScript`)