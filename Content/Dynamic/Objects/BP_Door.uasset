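; BP_Door is an interactable door that swings open and closed.
; Each Interaction event plays a pickup sound and flips a FlipFlop between playing and reversing a timeline, which lerps the Door's relative yaw for the swing.
; GetInteractionName returns InteractionArea, while GetInteractionWidgetRef returns nothing.
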(event `/Game/Dynamic/Interaction/BPI_Interaction.Interaction`
  (`GameplayStatics.PlaySoundAtLocation` "/Engine/VREditor/Sounds/UI/Object_PickUp.Object_PickUp" (0.0 0.0 240.0) (struct) 1.0 1.0 0.0 null null null null)
  (`/Engine/EditorBlueprintResources/StandardMacros.FlipFlop`
    (:`A`
      (bind (_direction _doorfloat) (`Timeline|OpenDoor Timeline` :!via `PlayFromStart` :!label _label)
        (:`Update`
          (`SceneComponent.K2_SetRelativeRotation` (`self.Door`) (`KismetMathLibrary.MakeRotator` 0.0 0.0 (`KismetMathLibrary.Lerp` 0.0 -95.0 _doorfloat)) false false))))
    (:`B`
      (goto _label :!via `Reverse`))))

(fn `GetInteractionName`
  (returns (InteractionName :type String))
  (return (`self.InteractionArea`)))

(fn `GetInteractionWidgetRef`
  (returns (Ref :type "WidgetComponent Object Reference"))
  (return null))

(fn `UserConstructionScript`)