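; BP_Note is an interactable note the player picks up to read and lays back down, highlighted through custom depth when focused.
; A FlipFlop on Interaction alternates between showing a note widget with the mesh hidden and look/move input locked, and laying it down to restore both.
; Picking it up also tells BP_FirstPersonGameMode to show the task list and flag it as shown.
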(event `self.ReceiveBeginPlay`)

(event `/Game/Dynamic/Interaction/BPI_Interaction.Interface_ToggleFocus`
  (params (Focus :type Boolean))
  (`PrimitiveComponent.SetRenderCustomDepth` (`self.Note`) Focus))

(event `self.Interaction`
  (bind _returnvalue (`GameplayStatics.GetPlayerController` 0))
  (bind _note (`self.Note`))
  (bind _returnvalue_2 (`SceneComponent.K2_GetComponentLocation` (`self.Note`)))
  (`/Engine/EditorBlueprintResources/StandardMacros.FlipFlop`
    (:`A`
      (`GameplayStatics.PlaySoundAtLocation` "/Engine/VREditor/Sounds/UI/Object_PickUp.Object_PickUp" _returnvalue_2 (struct) 1.0 1.0 0.0 null null null null)
      (bind _returnvalue_3 (`|CreateWidget` "/Game/Dynamic/Notes/WBP_NoteWidget.WBP_NoteWidget_C"))
      (bind _output_get (set `self.NoteWidgetRef` _returnvalue_3))
      (`/Game/Dynamic/Notes/WBP_NoteWidget.SetNoteImg` (`self.NoteWidgetRef`))
      (`UserWidget.AddToViewport` _output_get 0)
      (`Controller.SetIgnoreLookInput` _returnvalue true)
      (`Controller.SetIgnoreMoveInput` _returnvalue true)
      (`SceneComponent.SetVisibility` _note false false)
      (bind _asbp_first_person_game_mode (cast `/Game/Dynamic/FirstPerson/Blueprints/BP_FirstPersonGameMode` (`GameplayStatics.GetGameMode`)))
      (`/Game/Dynamic/FirstPerson/Blueprints/BP_FirstPersonGameMode.ShowTaskList` _asbp_first_person_game_mode)
      (set `/Game/Dynamic/FirstPerson/Blueprints/BP_FirstPersonGameMode.bTaskListShown` true _asbp_first_person_game_mode))
    (:`B`
      (`GameplayStatics.PlaySoundAtLocation` "/Engine/VREditor/Sounds/UI/Object_PickUp.Object_PickUp" _returnvalue_2 (struct) 1.0 1.0 0.0 null null null null)
      (`|CreateWidget` "/Game/Dynamic/UI/WBP_TaskList.WBP_TaskList_C")
      (`/Game/Dynamic/Notes/WBP_NoteWidget.LayNote Down` _returnvalue_3)
      (`Controller.SetIgnoreLookInput` _returnvalue false)
      (`Controller.SetIgnoreMoveInput` _returnvalue false)
      (`SceneComponent.SetVisibility` _note true false))))

(fn `GetInteractionName`
  (returns (InteractionName :type String))
  (return (`self.InteractionArea`)))

(fn `GetInteractionWidgetRef`
  (returns (Ref :type "WidgetComponent Object Reference"))
  (return null))

(fn `UserConstructionScript`)