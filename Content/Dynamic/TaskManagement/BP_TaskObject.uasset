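; BP_TaskObject is a task in the task management system that tracks progress toward a target count.
; IncrementCount adds an amount to the current count, clamped between zero and the target.
; It sets the completed flag when the count reaches the target, clears it otherwise, and triggers the task-updated notification in both cases.
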(fn `IncrementCount`
  (params (Amount :type Integer :default 1))
  (bind _targetcount (`self.TargetCount`))
  (bind _output_get (set `self.CurrentCount` (`KismetMathLibrary.Clamp` (+ (`self.CurrentCount`) Amount) 0 _targetcount)))
  (if (>= _output_get _targetcount)
    (set `self.bCompleted` true)
    (`self.onTaskUpdated`)
    (else
      (set `self.bCompleted` false)
      (`self.onTaskUpdated`))))