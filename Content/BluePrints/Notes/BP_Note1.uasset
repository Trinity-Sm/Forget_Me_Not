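; BP_Note1 is a note object that the player picks up to read and puts back down through an Interaction event.
; A FlipFlop alternates the two states, each playing a pickup sound at the note's location.
; Picking up shows a WBP_NoteWidget on screen, hides the note mesh and ignores player look and move input.
; Putting down calls LayNoteDown on that widget, restores input and makes the note visible again.
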(event `/Game/BluePrints/Interaction/BPI_Interaction.Interaction`
  (bind _returnvalue (`GameplayStatics.GetPlayerController` 0))
  (bind _note (`self.Note`))
  (bind _returnvalue_2 (`SceneComponent.K2_GetComponentLocation` (`self.Note`)))
  (`/Engine/EditorBlueprintResources/StandardMacros.FlipFlop`
    (:`A`
      (`GameplayStatics.PlaySoundAtLocation` "/Engine/VREditor/Sounds/UI/Object_PickUp.Object_PickUp" _returnvalue_2 (struct) 1.0 1.0 0.0 null null null null)
      (bind _returnvalue_3 (`|CreateWidget` "/Game/BluePrints/Notes/WBP_NoteWidget.WBP_NoteWidget_C"))
      (`UserWidget.AddToViewport` _returnvalue_3 0)
      (`Controller.SetIgnoreLookInput` _returnvalue true)
      (`Controller.SetIgnoreMoveInput` _returnvalue true)
      (`SceneComponent.SetVisibility` _note false false))
    (:`B`
      (`GameplayStatics.PlaySoundAtLocation` "/Engine/VREditor/Sounds/UI/Object_PickUp.Object_PickUp" _returnvalue_2 (struct) 1.0 1.0 0.0 null null null null)
      (`/Game/BluePrints/Notes/WBP_NoteWidget.LayNote Down` _returnvalue_3)
      (`Controller.SetIgnoreLookInput` _returnvalue false)
      (`Controller.SetIgnoreMoveInput` _returnvalue false)
      (`SceneComponent.SetVisibility` _note true false))))

(fn `UserConstructionScript`)